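; BP_JumpBoostCube is a placeable volume that boosts the first-person player's jump while they stand inside it.
; On BeginPlay it casts player character 0 to BP_FirstPersonCharacter and caches the reference.
; Its collision box calls AddJumpBoost with a configurable velocity multiplier on overlap begin and RemoveJumpBoost on overlap end, reacting only to that cached player.
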(event `self.ReceiveBeginPlay`
  (bind _asbp_first_person_character (cast `/Game/FirstPerson/Blueprints/BP_FirstPersonCharacter` (`GameplayStatics.GetPlayerCharacter` 0)))
  (set `self.PlayerCharRef` _asbp_first_person_character))

(event `self.JumpBoostCollisionBox.OnComponentBeginOverlap`
  (params (OverlappedComponent :type "PrimitiveComponent Object Reference") (OtherActor :type "Actor Object Reference") (OtherComp :type "PrimitiveComponent Object Reference") (OtherBodyIndex :type Integer) (bFromSweep :type Boolean) (SweepResult :type "HitResult Structure (by ref)"))
  (if (== OtherActor (`self.PlayerCharRef`))
    (`/Game/FirstPerson/Blueprints/BP_FirstPersonCharacter.AddJumpBoost` (`self.PlayerCharRef`) (`self.JumpBoostVelocityMultiplier`))))

(event `self.JumpBoostCollisionBox.OnComponentEndOverlap`
  (params (OverlappedComponent :type "PrimitiveComponent Object Reference") (OtherActor :type "Actor Object Reference") (OtherComp :type "PrimitiveComponent Object Reference") (OtherBodyIndex :type Integer))
  (if (== OtherActor (`self.PlayerCharRef`))
    (`/Game/FirstPerson/Blueprints/BP_FirstPersonCharacter.RemoveJumpBoost` (`self.PlayerCharRef`))))

(fn `UserConstructionScript`)