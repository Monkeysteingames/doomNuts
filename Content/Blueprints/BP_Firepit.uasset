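; BP_Firepit is a firepit actor that provides fire audio and flickering light.
; On BeginPlay it plays the Fire sound once at the static mesh's location with small ambient attenuation, then starts a flicker timeline.
; Each timeline update adds the curve value to a base intensity and applies the result to both point lights, so they flicker in sync.
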(event `self.ReceiveBeginPlay`
  (`GameplayStatics.PlaySoundAtLocation` "/Game/SFX_Music/SFX/Fire.Fire" (`SceneComponent.K2_GetComponentLocation` (`self.StaticMesh`)) (struct) 1.0 1.0 0.0 "/Game/SFX_Music/SFX/SmallAmbientAttenuation.SmallAmbientAttenuation" null null null)
  (bind (_direction _lightintensityfloatvalue) (`Timeline|LightFlickerTimeline` :!via `PlayFromStart`)
    (:`Update`
      (`LightComponent.SetIntensity` (`self.PointLight`) (+ (`self.BaseLightIntensity`) _lightintensityfloatvalue))
      (`LightComponent.SetIntensity` (`self.PointLight1`) (+ (`self.BaseLightIntensity`) _lightintensityfloatvalue)))))

(fn `UserConstructionScript`)