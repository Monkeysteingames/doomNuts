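; BP_Laser is a moving laser hazard that respawns the player's first-person character.
; On BeginPlay it adds a relative InterpToMovement control point and attaches a beam particle to its mesh.
; Each Tick it line-traces from the mesh along the world X axis, ends the beam at the hit location and spawns a hit effect there.
; A BP_FirstPersonCharacter check then triggers RespawnPlayer on player 0.
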(event `self.ReceiveBeginPlay`
  (`InterpToMovementComponent.AddControlPointPosition` (`self.InterpToMovement`) (`self.InterpDistance`) true)
  (bind _returnvalue (`GameplayStatics.SpawnEmitterAttached` "/Game/ParticleSystems/PS_Laser.PS_Laser" (`self.StaticMesh`)))
  (set `self.Laser` _returnvalue))

(event `self.ReceiveTick`
  (params (DeltaSeconds :type "Float (single-precision)"))
  (bind _returnvalue_x (`KismetMathLibrary.BreakVector` (* (0.0 0.0 0.0) 5000.0)))
  (bind _outsourcepoint (`ParticleSystemComponent.GetBeamSourcePoint` (`self.Laser`) 0 0))
  (`ParticleSystemComponent.SetBeamSourcePoint` (`self.Laser`) 0 (`SceneComponent.K2_GetComponentLocation` (`self.StaticMesh`)) 0)
  (bind _outhit (`KismetSystemLibrary.LineTraceSingle` (`KismetMathLibrary.MakeVector` (.x _outsourcepoint) (.y _outsourcepoint) (.z _outsourcepoint)) (`KismetMathLibrary.MakeVector` _returnvalue_x (.y _outsourcepoint) (.z _outsourcepoint)) "TraceTypeQuery1" true))
  (`ParticleSystemComponent.SetBeamEndPoint` (`self.Laser`) 0 (`.Location` (`GameplayStatics.BreakHitResult` _outhit)))
  (`GameplayStatics.SpawnEmitterAtLocation` "/Game/ParticleSystems/PS_LaserHit.PS_LaserHit" (`.Location` (`GameplayStatics.BreakHitResult` _outhit)))
  (if (== null "/Game/FirstPerson/Blueprints/BP_FirstPersonCharacter.BP_FirstPersonCharacter")
    (bind _asbp_first_person_character (cast `/Game/FirstPerson/Blueprints/BP_FirstPersonCharacter` (`GameplayStatics.GetPlayerCharacter` 0)))
    (`/Game/FirstPerson/Blueprints/BP_FirstPersonCharacter.RespawnPlayer` _asbp_first_person_character)))

(fn `UserConstructionScript`)