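; BP_TVLobby is a TV lobby actor with flickering lights and a one-time sound trigger.
; On BeginPlay, a timeline plays and drives both point lights, adding its float track to a base intensity on each update.
; The first overlap with the Box component plays the Lets_Lobby 2D sound through a DoOnce, with no check on the overlapping actor.
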(event `self.ReceiveBeginPlay`
  (bind (_direction _lightintensityfloatvalue) (`Timeline|LightFlickerTimeline`)
    (:`Update`
      (`LightComponent.SetIntensity` (`self.PointLight`) (+ (`self.BaseLightIntensity`) _lightintensityfloatvalue))
      (`LightComponent.SetIntensity` (`self.PointLight1`) (+ (`self.BaseLightIntensity`) _lightintensityfloatvalue)))))

(event `self.Box.OnComponentBeginOverlap`
  (params (OverlappedComponent :type "PrimitiveComponent Object Reference") (OtherActor :type "Actor Object Reference") (OtherComp :type "PrimitiveComponent Object Reference") (OtherBodyIndex :type Integer) (bFromSweep :type Boolean) (SweepResult :type "HitResult Structure (by ref)"))
  (if true
    (`/Engine/EditorBlueprintResources/StandardMacros.DoOnce` false
      (:`Completed`
        (`GameplayStatics.PlaySound2D` "/Game/SFX_Music/Music/Lets_Lobby.Lets_Lobby" 1.0 1.0 0.0 null null)))))

(fn `UserConstructionScript`)