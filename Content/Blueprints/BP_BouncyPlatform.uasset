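; Bouncy platform that bobs vertically when the first-person player character hits it from above or below, then settles back.
; Top and bottom trigger boxes each play a timeline that nudges the root's Z incrementally every update, with opposite signs.
; A shared cooldown blocks retriggering until the timeline finishes, when the root eases back to the location cached at BeginPlay.
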(event `self.ReceiveBeginPlay`
  (bind _asbp_first_person_character (cast `/Game/FirstPerson/Blueprints/BP_FirstPersonCharacter` (`GameplayStatics.GetPlayerCharacter` 0)))
  (set `self.PlayerCharacterRef` _asbp_first_person_character)
  (set `self.BaseWorldLocation` (`SceneComponent.K2_GetComponentLocation` (`self.DefaultSceneRoot`))))

(event `self.TopBangBox.OnComponentBeginOverlap`
  (params (OverlappedComponent :type "PrimitiveComponent Object Reference") (OtherActor :type "Actor Object Reference") (OtherComp :type "PrimitiveComponent Object Reference") (OtherBodyIndex :type Integer) (bFromSweep :type Boolean) (SweepResult :type "HitResult Structure (by ref)"))
  (bind _defaultsceneroot (`self.DefaultSceneRoot`))
  (bind (_returnvalue_x _returnvalue_y _returnvalue_z) (`KismetMathLibrary.BreakVector` (`SceneComponent.K2_GetComponentLocation` _defaultsceneroot)))
  (if (== OtherActor (`self.PlayerCharacterRef`))
    (if (not (`self.OnCooldown`))
      (set `self.OnCooldown` true)
      (bind (_direction _floatnegative) (`Timeline|Timeline` :!via `PlayFromStart`)
        (:`Update`
          (`SceneComponent.K2_SetWorldLocation` _defaultsceneroot (`KismetMathLibrary.MakeVector` _returnvalue_x _returnvalue_y (+ _returnvalue_z _floatnegative)) false false))
        (:`Finished`
          (set `self.OnCooldown` false)
          (`KismetSystemLibrary.MoveComponentTo` (`self.DefaultSceneRoot`) (`self.BaseWorldLocation`) (struct) false false 0.1))))))

(event `self.BottomBangBox.OnComponentBeginOverlap`
  (params (OverlappedComponent :type "PrimitiveComponent Object Reference") (OtherActor :type "Actor Object Reference") (OtherComp :type "PrimitiveComponent Object Reference") (OtherBodyIndex :type Integer) (bFromSweep :type Boolean) (SweepResult :type "HitResult Structure (by ref)"))
  (bind _defaultsceneroot (`self.DefaultSceneRoot`))
  (bind (_returnvalue_x _returnvalue_y _returnvalue_z) (`KismetMathLibrary.BreakVector` (`SceneComponent.K2_GetComponentLocation` _defaultsceneroot)))
  (if (== OtherActor (`self.PlayerCharacterRef`))
    (if (not (`self.OnCooldown`))
      (set `self.OnCooldown` true)
      (bind (_direction _floatnegative) (`Timeline|Timeline_0` :!via `PlayFromStart`)
        (:`Update`
          (`SceneComponent.K2_SetWorldLocation` _defaultsceneroot (`KismetMathLibrary.MakeVector` _returnvalue_x _returnvalue_y (- _returnvalue_z _floatnegative)) false false))
        (:`Finished`
          (set `self.OnCooldown` false)
          (`KismetSystemLibrary.MoveComponentTo` (`self.DefaultSceneRoot`) (`self.BaseWorldLocation`) (struct) false false 0.1))))))

(fn `UserConstructionScript`)