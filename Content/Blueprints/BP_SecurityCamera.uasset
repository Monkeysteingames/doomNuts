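; BP_SecurityCamera is a security camera that reacts when the first-person player character enters its capsule detection volume.
; On overlap it plays an alarm, turns its spotlight magenta and swaps a glass material on the mesh to blue.
; One second after the player leaves, the light and glass switch to green.
; It also plays a camera noise at the mesh's location on BeginPlay.
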(event `self.ReceiveBeginPlay`
  (`GameplayStatics.PlaySoundAtLocation` "/Game/SFX_Music/SFX/SecurityCamNoise.SecurityCamNoise" (`SceneComponent.K2_GetComponentLocation` (`self.StaticMesh`)) (struct) 1.0 1.0 0.0 "/Game/SFX_Music/SFX/SmallAmbientAttenuation.SmallAmbientAttenuation" null null null))

(event `self.Capsule.OnComponentBeginOverlap`
  (params (OverlappedComponent :type "PrimitiveComponent Object Reference") (OtherActor :type "Actor Object Reference") (OtherComp :type "PrimitiveComponent Object Reference") (OtherBodyIndex :type Integer) (bFromSweep :type Boolean) (SweepResult :type "HitResult Structure (by ref)"))
  (cast `/Game/FirstPerson/Blueprints/BP_FirstPersonCharacter` OtherActor)
  (`GameplayStatics.PlaySoundAtLocation` "/Game/SFX_Music/SFX/Alarm_02.Alarm_02" (`SceneComponent.K2_GetComponentLocation` (`self.Capsule`)) (struct) 1.0 1.0 0.0 "/Game/SFX_Music/SFX/SmallAmbientAttenuation.SmallAmbientAttenuation" null null null)
  (`LightComponent.SetLightColor` (`self.SpotLight`) (struct :`R` 0.869181 :`B` 0.954167 :`A` 1.0) true)
  (`PrimitiveComponent.SetMaterial` (`self.StaticMesh`) 4 "/Game/Textures/Base_Colors/Color_Blue_Glass.Color_Blue_Glass"))

(event `self.Capsule.OnComponentEndOverlap`
  (params (OverlappedComponent :type "PrimitiveComponent Object Reference") (OtherActor :type "Actor Object Reference") (OtherComp :type "PrimitiveComponent Object Reference") (OtherBodyIndex :type Integer))
  (cast `/Game/FirstPerson/Blueprints/BP_FirstPersonCharacter` OtherActor)
  (`KismetSystemLibrary.Delay` 1.0)
  (`LightComponent.SetLightColor` (`self.SpotLight`) (struct :`G` 1.0 :`A` 1.0) true)
  (`PrimitiveComponent.SetMaterial` (`self.StaticMesh`) 4 "/Game/Textures/Base_Colors/Color_Green_Glass.Color_Green_Glass"))

(fn `UserConstructionScript`)