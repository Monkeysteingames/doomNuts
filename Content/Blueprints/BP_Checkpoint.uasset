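; BP_Checkpoint is a trigger actor that records itself as the player's most recent checkpoint.
; BeginPlay caches the first-person player character, cast to BP_FirstPersonCharacter.
; When that character overlaps the collision box, the checkpoint writes itself into the character's RecentCheckpointRef and sets its PassedCheckpoint flag.
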(event `self.ReceiveBeginPlay`
  (bind _asbp_first_person_character (cast `/Game/FirstPerson/Blueprints/BP_FirstPersonCharacter` (`GameplayStatics.GetPlayerCharacter` 0)))
  (set `self.PlayerCharRef` _asbp_first_person_character))

(event `self.ReceiveTick`
  (params (DeltaSeconds :type "Float (single-precision)")))

(event `self.CheckpointCollisionBox.OnComponentBeginOverlap`
  (params (OverlappedComponent :type "PrimitiveComponent Object Reference") (OtherActor :type "Actor Object Reference") (OtherComp :type "PrimitiveComponent Object Reference") (OtherBodyIndex :type Integer) (bFromSweep :type Boolean) (SweepResult :type "HitResult Structure (by ref)"))
  (bind _playercharref (`self.PlayerCharRef`))
  (if (== OtherActor (`self.PlayerCharRef`))
    (set `/Game/FirstPerson/Blueprints/BP_FirstPersonCharacter.RecentCheckpointRef` null (`self.PlayerCharRef`))
    (set `/Game/FirstPerson/Blueprints/BP_FirstPersonCharacter.RecentCheckpointRef` self (`self.PlayerCharRef`))
    (if (not (`/Game/FirstPerson/Blueprints/BP_FirstPersonCharacter.bPassedCheckpoint` _playercharref))
      (set `/Game/FirstPerson/Blueprints/BP_FirstPersonCharacter.bPassedCheckpoint` true _playercharref))))

(fn `UserConstructionScript`)